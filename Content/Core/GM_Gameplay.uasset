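; Gameplay game mode that runs a timed match between Blue and Red teams and keeps their scores.
; On BeginPlay it creates the score widget and starts a looping timer that sends the remaining minutes, derived from game time, to it.
; AddScore increments the chosen team's score and updates the widget.
; Match end is only a placeholder debug print, with an unconnected ResetLevel call.
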(event Custom|TimerCountdown
  (bind _returnvalue (Utilities|Time|GetTimeSeconds))
  (bind _matchtotaltimeinseconds (Variables|Default|GetMatchTotalTimeInSeconds))
  (bind _returnvalue_2 (- _matchtotaltimeinseconds _returnvalue))
  (bind _returnvalue_3 (/ _returnvalue_2 6e+01))
  ;[1 1 1] Match countdown timer
  (Math|Float|CompareFloat _returnvalue_3 0.0
    (:>
      (Default|SetTimerText (Variables|Default|GetWidgetScoreReference) _returnvalue_3))
    (:==
      (Development|PrintString "Hello" :!label _label))
    (:<
      (goto _label))))

(event EventBeginPlay
  (bind _returnvalue (UserInterface|CreateWidget "/Game/UI/WBP_Score.WBP_Score_C"))
  (bind _output_get (Variables|Default|SetWidgetScoreReference _returnvalue))
  (UserInterface|Viewport|AddtoViewport _output_get 0)
  (Utilities|Time|SetTimerbyFunctionName 0 "TimerCountdown" (Variables|Default|GetTimerTickRate) true))

(event EventAddScore
  (params (IsBlueTeam? :type Boolean))
  (bind _widgetscorereference (Variables|Default|GetWidgetScoreReference))
  ;[1 1 1] Adding Score
  (if IsBlueTeam?
    (bind _result (Math|Integer|IncrementInt (Variables|Default|GetBlueTeamScore))
      (:%20%20
        (bind _output_get (Variables|Default|SetBlueTeamScore _result))
        (Default|BlueTeamAddScore _widgetscorereference _output_get)))
    (else
      (bind _result_2 (Math|Integer|IncrementInt (Variables|Default|GetRedTeamScore))
        (:%20%20
          (bind _output_get_2 (Variables|Default|SetRedTeamScore _result_2))
          (Default|RedTeamAddScore _widgetscorereference _output_get_2))))))

(fn ConstructionScript)