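; Player controller for Turtle Tanks that handles pausing and resuming the game.
; BeginPlay creates the pause menu widget once and caches it for reuse.
; PauseGame input pauses an unpaused game, while the ResumeGame event unpauses it.
; Both feed MouseCursorFocus, which toggles the cursor, switches between UI-only and game-only input, and adds or removes the menu.
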(event Custom|ResumeGame
  ;[1 1 1] Pause Game
  (Game|SetGamePaused false)
  (CallFunction|MouseCursor&Focus (Game|IsGamePaused)))

(event EventBeginPlay
  (bind _returnvalue (UserInterface|CreateWidget "/Game/UI/WBP_PauseMenu.WBP_PauseMenu_C"))
  (Variables|Default|SetWBP_PauseReference _returnvalue))

(event Input|ActionEvents|InputActionPauseGame
  (params (Key :type Key%20Structure :default "None"))
  ;[1 1 1] Pause Game
  (:Pressed
    (if (not (Game|IsGamePaused))
      (bind _returnvalue (Game|SetGamePaused true))
      (CallFunction|MouseCursor&Focus _returnvalue))))

(fn ConstructionScript)

(fn MouseCursor&Focus
  (params (bShowMouseCursor :type Boolean))
  (bind _self self)
  (bind _wbp_pausereference (Variables|Default|GetWBP_PauseReference))
  (bind _output_get (Variables|Default|SetbShowMouseCursor bShowMouseCursor))
  (if _output_get
    (Input|SetInputModeUIOnly _self _wbp_pausereference "DoNotLock")
    (UserInterface|Viewport|AddtoViewport _wbp_pausereference 0)
    (else
      (Input|SetInputModeGameOnly _self)
      (Widget|RemovefromParent _wbp_pausereference))))